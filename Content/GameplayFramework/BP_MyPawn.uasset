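; Player pawn for a strategy game that moves on input axes and places units by mouse click, with cursor and in-game HUD set up at BeginPlay.
; A click traces under the cursor and, for overlapped BP_Zonadejuego actors, deducts the selected cost from Dinero if affordable.
; It then spawns a BP_Campamento configured for soldier, ram or medic, or a defensive tower directly.
; Dinero compounds every Tick, so income depends on frame rate.
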(event EventBeginPlay
  (bind _returnvalue (Game|GetPlayerController 0))
  (Variables|/Script/Engine.PlayerController|SetbShowMouseCursor _returnvalue true)
  (Input|SetInputModeGameandUI _returnvalue 0 "DoNotLock" false false)
  (bind _returnvalue_2 (UserInterface|CreateWidget "/Game/UI/WG_InGame.WG_InGame_C"))
  (UserInterface|Viewport|AddtoViewport _returnvalue_2 0))

(event EventTick
  (params (DeltaSeconds :type Float%20%28single-precision%29))
  (Variables|Default|SetDinero (* (Variables|Default|GetDinero) 1.0001)))

(event Input|AxisEvents|InputAxisMoverAdelanteAtras
  (params (AxisValue :type Float%20%28single-precision%29))
  (Pawn|Input|AddMovementInput (Transformation|GetActorForwardVector) AxisValue false))

(event Input|AxisEvents|InputAxisMoverDerechaIzquierda
  (params (AxisValue :type Float%20%28single-precision%29))
  (Pawn|Input|AddMovementInput (Transformation|GetActorRightVector) AxisValue false))

(event Input|MouseEvents|LeftMouseButton
  (params (Key :type Key%20Structure :default "None"))
  (bind _returnvalue (Game|GetPlayerController 0))
  (bind _hitresult (Game|Player|GetHitResultUnderCursorbyChannel _returnvalue "TraceTypeQuery1" true))
  (bind (_bblockinghit _binitialoverlap _time _distance _location) (Collision|BreakHitResult _hitresult))
  (bind _returnvalue_2 (+ _location "0.000000,0.000000,100.000000"))
  (bind _returnvalue_3 (Math|Transform|MakeTransform _returnvalue_2))
  (:Pressed
    (if _bblockinghit
      (bind _outactors (Collision|SphereOverlapActors _location 0.0 (Utilities|Array|MakeArray "ObjectTypeQuery2") 0))
      (for _array_element _outactors
        (Utilities|Casting|CastToBP_Zonadejuego _array_element)
        (if (>= (Variables|Default|GetDinero) (Variables|Default|GetCosteUnidadSeleccionada))
          (Variables|Default|SetDinero (- (Variables|Default|GetDinero) (Variables|Default|GetCosteUnidadSeleccionada)))
          (switch Utilities|FlowControl|Switch|SwitchonEnum_Unidad (Variables|Default|GetUnidadSeleccionada)
            (:NewEnumerator0
              (Game|SpawnActorfromClass "/Game/Blueprints/BP_Campamento.BP_Campamento_C" _returnvalue_3 "Undefined" "MultiplyWithRoot" 0 "/Game/Blueprints/BP_Soldado.BP_Soldado_C" "NewEnumerator0" 0))
            (:NewEnumerator1
              (Game|SpawnActorfromClass "/Game/Blueprints/BP_Campamento.BP_Campamento_C" _returnvalue_3 "Undefined" "MultiplyWithRoot" 0 "/Game/Blueprints/BP_Ariete.BP_Ariete_C" "NewEnumerator0" 0))
            (:NewEnumerator2
              (Game|SpawnActorfromClass "/Game/Blueprints/BP_Campamento.BP_Campamento_C" _returnvalue_3 "Undefined" "MultiplyWithRoot" 0 "/Game/Blueprints/BP_Medico.BP_Medico_C" "NewEnumerator0" 0))
            (:NewEnumerator3
              (Game|SpawnActorfromClass "/Game/Blueprints/BP_TorreDefensiva.BP_TorreDefensiva_C" _returnvalue_3 "Undefined" "MultiplyWithRoot" 0 "NewEnumerator0" 0))))))))

(fn ConstructionScript)