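; BP_Agente is an AI-controlled agent with a health value that it displays as floating text.
; On possession by an AI controller, it runs its assigned behavior tree.
; Incoming damage is subtracted from Salud, and the actor destroys itself when that reaches zero or below.
; Every tick it refreshes the text and orients it from the player pawn's rotation with a 180-degree offset.
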(event EventPossessed
  (params (NewController :type Controller%20Object%20Reference))
  (bind _asaicontroller (Utilities|Casting|CastToAIController NewController))
  (AI|RunBehaviorTree _asaicontroller (Variables|Default|GetBTAsset)))

(event EventTick
  (params (DeltaSeconds :type Float%20%28single-precision%29))
  (bind _textrender (Variables|Default|GetTextRender))
  (Rendering|Components|TextRender|SetText _textrender (Utilities|Text|ToText(Float) (Variables|Default|GetSalud) "HalfToEven"))
  (Transformation|SetWorldRotation _textrender (Math|Rotator|CombineRotators (Transformation|GetActorRotation (Game|Player|GetPlayerPawn 0)) "0.000000,180.000000,0.000000") false false))

(event Game|Damage|EventAnyDamage
  (params (Damage :type Float%20%28single-precision%29) (DamageType :type Damage%20Type%20Object%20Reference) (InstigatedBy :type Controller%20Object%20Reference) (DamageCauser :type Actor%20Object%20Reference))
  (bind _output_get (Variables|Default|SetSalud (- (Variables|Default|GetSalud) Damage)))
  (if (<= _output_get 0.0)
    (Actor|DestroyActor)))

(fn ConstructionScript)