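; BP_Barricada is a barricade that hinders BP_Agente characters passing through its DamageBox overlap volume.
; Entering the box halves the agent's max walk speed and leaving restores it by dividing by the same factor.
; On entry, agents whose Faccion differs from the barricade's also take a fixed amount of damage, while the slowdown applies to every faction.
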(event OnComponentBeginOverlap(DamageBox)
  (params (OverlappedComponent :type Primitive%20Component%20Object%20Reference) (OtherActor :type Actor%20Object%20Reference) (OtherComp :type Primitive%20Component%20Object%20Reference) (OtherBodyIndex :type Integer) (bFromSweep :type Boolean) (SweepResult :type Hit%20Result%20Structure%20%28by%20ref%29))
  (bind _asbp_agente (Utilities|Casting|CastToBP_Agente OtherActor))
  (Variables|/Script/Engine.CharacterMovementComponent|SetMaxWalkSpeed (Variables|/Script/Engine.Character|GetCharacterMovement _asbp_agente) (* (Variables|/Script/Engine.CharacterMovementComponent|GetMaxWalkSpeed (Variables|/Script/Engine.Character|GetCharacterMovement _asbp_agente)) 0.5))
  (if (Utilities|Enum|NotEqual(Enum) (Variables|/Game/Blueprints/BP_Agente.BP_Agente_C|GetFaccion _asbp_agente) (Variables|Default|GetFaccion))
    (Game|Damage|ApplyDamage _asbp_agente 1e+01 0 0)))

(event OnComponentEndOverlap(DamageBox)
  (params (OverlappedComponent :type Primitive%20Component%20Object%20Reference) (OtherActor :type Actor%20Object%20Reference) (OtherComp :type Primitive%20Component%20Object%20Reference) (OtherBodyIndex :type Integer))
  (bind _asbp_agente (Utilities|Casting|CastToBP_Agente OtherActor))
  (Variables|/Script/Engine.CharacterMovementComponent|SetMaxWalkSpeed (Variables|/Script/Engine.Character|GetCharacterMovement _asbp_agente) (/ (Variables|/Script/Engine.CharacterMovementComponent|GetMaxWalkSpeed (Variables|/Script/Engine.Character|GetCharacterMovement _asbp_agente)) 0.5)))

(fn ConstructionScript)