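; BP_Carretera is a road zone actor that speeds up BP_Agente characters while they overlap it.
; On begin overlap it casts the other actor to BP_Agente and multiplies its CharacterMovement MaxWalkSpeed by 1.5.
; On end overlap it divides that speed by the same factor, so the boost is relative to the current speed rather than a stored base value.
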(event Collision|EventActorBeginOverlap
  (params (OtherActor :type Actor%20Object%20Reference))
  (bind _asbp_agente (Utilities|Casting|CastToBP_Agente OtherActor))
  (Variables|/Script/Engine.CharacterMovementComponent|SetMaxWalkSpeed (Variables|/Script/Engine.Character|GetCharacterMovement _asbp_agente) (* (Variables|/Script/Engine.CharacterMovementComponent|GetMaxWalkSpeed (Variables|/Script/Engine.Character|GetCharacterMovement _asbp_agente)) 1.5)))

(event Collision|EventActorEndOverlap
  (params (OtherActor :type Actor%20Object%20Reference))
  (bind _asbp_agente (Utilities|Casting|CastToBP_Agente OtherActor))
  (Variables|/Script/Engine.CharacterMovementComponent|SetMaxWalkSpeed (Variables|/Script/Engine.Character|GetCharacterMovement _asbp_agente) (/ (Variables|/Script/Engine.CharacterMovementComponent|GetMaxWalkSpeed (Variables|/Script/Engine.Character|GetCharacterMovement _asbp_agente)) 1.5)))

(fn ConstructionScript)