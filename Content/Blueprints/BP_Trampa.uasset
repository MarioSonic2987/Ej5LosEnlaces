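; BP_Trampa is a faction-owned trap that explodes when an agent of another faction steps on it.
; On Trigger overlap it casts to BP_Agente and compares Faccion, ignoring agents of its own faction.
; For other factions it destroys itself, spawns an explosion emitter at its location and applies fixed damage to the agent.
; The construction script tints the Plane through a dynamic material instance using the faction's color.
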(event OnComponentBeginOverlap(Trigger)
  (params (OverlappedComponent :type Primitive%20Component%20Object%20Reference) (OtherActor :type Actor%20Object%20Reference) (OtherComp :type Primitive%20Component%20Object%20Reference) (OtherBodyIndex :type Integer) (bFromSweep :type Boolean) (SweepResult :type Hit%20Result%20Structure%20%28by%20ref%29))
  (bind _asbp_agente (Utilities|Casting|CastToBP_Agente OtherActor))
  (if (Utilities|Enum|NotEqual(Enum) (Variables|/Game/Blueprints/BP_Agente.BP_Agente_C|GetFaccion _asbp_agente) (Variables|Default|GetFaccion))
    (Actor|DestroyActor)
    (Effects|SpawnEmitteratLocation "/Game/StarterContent/Particles/P_Explosion.P_Explosion" (Transformation|GetActorLocation))
    (Game|Damage|ApplyDamage _asbp_agente 25.0 0 0)))

(event EventBeginPlay)

(event Collision|EventActorBeginOverlap
  (params (OtherActor :type Actor%20Object%20Reference)))

(event EventTick
  (params (DeltaSeconds :type Float%20%28single-precision%29)))

(fn ConstructionScript
  (bind _returnvalue (Rendering|Material|CreateDynamicMaterialInstance (Variables|Default|GetPlane) 0 "/Engine/BasicShapes/BasicShapeMaterial.BasicShapeMaterial" "None" :!class /Script/Engine.PrimitiveComponent))
  (Rendering|Material|SetVectorParameterValue _returnvalue "Color" (CallFunction|GetColorFaccion (Variables|Default|GetFaccion)) :!class /Script/Engine.MaterialInstanceDynamic))